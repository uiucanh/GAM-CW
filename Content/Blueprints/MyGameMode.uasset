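; Game mode that sets up the level on start and tracks run time and player health.
; On BeginPlay it switches to unlit view mode via console command and starts background music.
; Tick adds delta time to a timer in MyGameInstance while it is running.
; ReduceHealth decrements health, playing a hurt sound, or calls ReduceLive on the game instance when health reaches zero.
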(event EventBeginPlay
  (Development|ExecuteConsoleCommand "viewmode unlit")
  (Audio|PlaySound2D "/Game/Sound/BackgroundMusicCue.BackgroundMusicCue"))

(event EventTick
  (params (DeltaSeconds :type Float%20%28single-precision%29))
  (bind _asmy_game_instance (Utilities|Casting|CastToMyGameInstance (Game|GetGameInstance)))
  (if (Variables|/Game/Blueprints/MyGameInstance.MyGameInstance_C|GetRunning _asmy_game_instance)
    (Variables|/Game/Blueprints/MyGameInstance.MyGameInstance_C|SetTimer _asmy_game_instance (+ (Variables|/Game/Blueprints/MyGameInstance.MyGameInstance_C|GetTimer _asmy_game_instance) DeltaSeconds))))

(fn ConstructionScript)

(fn ReduceHealth
  (bind _playerhealth (Variables|Default|GetPlayerHealth))
  (Math|Integer|DecrementInt _playerhealth
    (:%20%20
      (if (== _playerhealth 0)
        (bind _asmy_game_instance (Utilities|Casting|CastToMyGameInstance (Game|GetGameInstance)))
        (Default|ReduceLive _asmy_game_instance)
        (else
          (Audio|PlaySound2D "/Game/Sound/PlayerHurt_Cue.PlayerHurt_Cue"))))))