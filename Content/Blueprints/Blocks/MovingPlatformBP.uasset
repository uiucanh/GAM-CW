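; A moving platform block that travels between two relative points, PointA and PointB.
; The construction script feeds both points and Speed, used as the duration, into an InterpToMovement component.
; When the player pawn overlaps the Box, the RenderComponent is set to ignore that PlayerBP while moving.
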(event OnComponentBeginOverlap(Box)
  (params (OverlappedComponent :type Primitive%20Component%20Object%20Reference) (OtherActor :type Actor%20Object%20Reference) (OtherComp :type Primitive%20Component%20Object%20Reference) (OtherBodyIndex :type Integer) (bFromSweep :type Boolean) (SweepResult :type Hit%20Result%20Structure%20%28by%20ref%29))
  (bind _returnvalue (Game|Player|GetPlayerPawn 0))
  (if (== _returnvalue OtherActor)
    ;[1 1 1] Ignore player when moving
    (bind _asplayer_bp (Utilities|Casting|CastToPlayerBP _returnvalue))
    (Collision|IgnoreActorwhenMoving (Variables|Default|GetRenderComponent) _asplayer_bp true)))

(fn ConstructionScript
  (bind _interptomovement (Variables|Default|GetInterpToMovement))
  (Variables|/Script/Engine.InterpToMovementComponent|SetDuration _interptomovement (Variables|Default|GetSpeed))
  (Variables|/Script/Engine.InterpToMovementComponent|SetControlPoints _interptomovement (Utilities|Array|MakeArray (Utilities|Struct|MakeInterpControlPoint (Variables|Default|GetPoint%20A) true) (Utilities|Struct|MakeInterpControlPoint (Variables|Default|GetPoint%20B) true))))