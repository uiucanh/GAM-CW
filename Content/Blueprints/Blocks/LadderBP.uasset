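; LadderBP is a climbable ladder block that lets the player climb while inside its trigger box.
; When the first player's pawn enters the box, it casts to PlayerBP and sets CanClimb to true.
; When that pawn leaves, it clears CanClimb and calls EndClimbing, leaving the climbing itself to PlayerBP.
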(event OnComponentBeginOverlap(Box)
  (params (OverlappedComponent :type Primitive%20Component%20Object%20Reference) (OtherActor :type Actor%20Object%20Reference) (OtherComp :type Primitive%20Component%20Object%20Reference) (OtherBodyIndex :type Integer) (bFromSweep :type Boolean) (SweepResult :type Hit%20Result%20Structure%20%28by%20ref%29))
  (bind _returnvalue (Game|Player|GetPlayerPawn 0))
  (if (== _returnvalue OtherActor)
    (bind _asplayer_bp (Utilities|Casting|CastToPlayerBP _returnvalue))
    (Variables|/Game/Blueprints/PlayerBP.PlayerBP_C|SetcanClimb _asplayer_bp true)))

(event OnComponentEndOverlap(Box)
  (params (OverlappedComponent :type Primitive%20Component%20Object%20Reference) (OtherActor :type Actor%20Object%20Reference) (OtherComp :type Primitive%20Component%20Object%20Reference) (OtherBodyIndex :type Integer))
  (bind _returnvalue (Game|Player|GetPlayerPawn 0))
  (if (== _returnvalue OtherActor)
    (bind _asplayer_bp (Utilities|Casting|CastToPlayerBP _returnvalue))
    (Variables|/Game/Blueprints/PlayerBP.PlayerBP_C|SetcanClimb _asplayer_bp false)
    (Default|EndClimbing _asplayer_bp)))

(event EventBeginPlay)

(event Collision|EventActorBeginOverlap
  (params (OtherActor :type Actor%20Object%20Reference)))

(event EventTick
  (params (DeltaSeconds :type Float%20%28single-precision%29)))

(fn ConstructionScript)