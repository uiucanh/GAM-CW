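; DisappearingPlatformBP is a platform block that cycles between visible and vanished on a timer.
; Each Tick starts a Delay, using separate durations for the shown and hidden phases.
; When a delay ends, it toggles the actor's hidden state, RenderComponent collision and the Disappered flag together, so the hidden platform cannot be stood on.
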(event EventTick
  (params (DeltaSeconds :type Float%20%28single-precision%29))
  (if (Variables|Default|GetDisappered)
    (Utilities|FlowControl|Delay (Variables|Default|GetDisappear%20Time))
    (Rendering|SetActorHiddenInGame false)
    (Collision|SetCollisionEnabled (Variables|Default|GetRenderComponent) "QueryAndPhysics")
    (Variables|Default|SetDisappered false)
    (else
      (Utilities|FlowControl|Delay (Variables|Default|GetAppear%20Time))
      (Rendering|SetActorHiddenInGame true)
      (Collision|SetCollisionEnabled (Variables|Default|GetRenderComponent) "NoCollision")
      (Variables|Default|SetDisappered true))))

(fn ConstructionScript)