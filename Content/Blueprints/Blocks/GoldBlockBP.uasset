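; GoldBlockBP is a hittable coin block that rewards the player with coins until it runs empty.
; When the player pawn hits its Box, it decrements its coin count, spawns a CoinBP above itself and calls AddCoin on MyGameInstance.
; Once out of coins it swaps to the empty sprite and disables Box collision.
; Each spawned coin is destroyed after a short delay.
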(event OnComponentHit(Box)
  (params (HitComponent :type Primitive%20Component%20Object%20Reference) (OtherActor :type Actor%20Object%20Reference) (OtherComp :type Primitive%20Component%20Object%20Reference) (NormalImpulse :type Vector :default "0, 0, 0") (Hit :type Hit%20Result%20Structure%20%28by%20ref%29))
  (bind _returnvalue (Transformation|GetActorLocation))
  ;[1 1 1] When player hits the block, switch the sprite and disable the collision detection
  (if (== OtherActor (Game|Player|GetPlayerPawn 0))
    (Math|Integer|DecrementInt (Variables|Default|GetNumOfCoinsInBox)
      (:%20%20
        ;;[1 1 1] Spawn coin and add 1 to score
        (bind _returnvalue_2 (Game|SpawnActorfromClass "/Game/Blueprints/Objects/CoinBP.CoinBP_C" (Math|Conversions|ToTransform(Vector) (Math|Vector|MakeVector (.x _returnvalue) (.y _returnvalue) (+ (.z _returnvalue) 8e+01))) "Undefined" 0 0))
        (bind _asmy_game_instance (Utilities|Casting|CastToMyGameInstance (Game|GetGameInstance)))
        (Default|AddCoin _asmy_game_instance)
        (if (< (Variables|Default|GetNumOfCoinsInBox) 1)
          ;;[1 1 1] Change sprite and disable collision if out of coins
          (Rendering|Components|Sprite|SetSprite (Variables|Default|GetRenderComponent) "/Game/Art/Textures/Objects/boxEmpty_Sprite.boxEmpty_Sprite")
          (Collision|SetCollisionEnabled (Variables|Default|GetBox) "NoCollision"))
        (Utilities|FlowControl|Delay 0.5)
        (Actor|DestroyActor _returnvalue_2)))))

(event EventBeginPlay)

(event Collision|EventActorBeginOverlap
  (params (OtherActor :type Actor%20Object%20Reference)))

(event EventTick
  (params (DeltaSeconds :type Float%20%28single-precision%29)))

(fn ConstructionScript)