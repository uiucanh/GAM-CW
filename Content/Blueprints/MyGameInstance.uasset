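; Game instance that holds the player's coins, lives, timer and running state for a platformer-style game.
; AddCoin plays a sound and grants an extra life every ten coins.
; ReduceLive asks MyGameMode to restart while lives remain; at zero it stops and hides PlayerBP, then shows the GameOverScreen widget and mouse cursor.
; RestartTheGame reloads Level1 and resets all tracked values.
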(fn AddCoin
  (bind _numcoins (Variables|Default|GetNumCoins))
  ;[1 1 1] Add coin function, every 10 coins add 1 live
  (Math|Integer|IncrementInt _numcoins
    (:%20%20
      (Audio|PlaySound2D "/Game/Sound/coin.coin")
      (if (== (.Remainder (Math|Float|Division(WholeandRemainder) (Math|Conversions|ToFloat(Integer) _numcoins) 1e+01)) 0.0)
        (Math|Integer|IncrementInt (Variables|Default|GetNumLives)
          (:%20%20
            (Audio|PlaySound2D "/Game/Sound/item_pickup.item_pickup")))))))

(fn ReduceLive
  (bind _numlives (Variables|Default|GetNumLives))
  (Math|Integer|DecrementInt _numlives
    (:%20%20
      (if (== _numlives 0)
        (Variables|Default|SetRunning false)
        (bind _asplayer_bp (Utilities|Casting|CastToPlayerBP (Game|Player|GetPlayerPawn 0)))
        (Pawn|Components|CharacterMovement|SetMovementMode (Variables|/Script/Engine.Character|GetCharacterMovement _asplayer_bp) "MOVE_None" 0)
        (Rendering|SetVisibility (Variables|/Script/Paper2D.PaperCharacter|GetSprite _asplayer_bp) false false)
        (bind _returnvalue (UserInterface|CreateWidget "/Game/Blueprints/HUDs/GameOverScreen.GameOverScreen_C"))
        (UserInterface|Viewport|AddtoViewport _returnvalue 0)
        (Variables|/Script/Engine.PlayerController|SetbShowMouseCursor (Game|GetPlayerController 0) true)
        (else
          (bind _asmy_game_mode (Utilities|Casting|CastToMyGameMode (Game|GetGameMode)))
          (Class|GameMode|RestartGame _asmy_game_mode))))))

(fn RestarttheGame
  (Game|OpenLevel(byName) "Level1")
  (Variables|Default|SetNumCoins 0)
  (Variables|Default|SetTimer 0.0)
  (Variables|Default|SetNumLives 3)
  (Variables|Default|SetRunning true))