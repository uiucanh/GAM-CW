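; Saw hazard that moves between two points, knocking back and damaging the player on contact.
; The construction script builds the InterpToMovement path from relative PointA and PointB, using Speed as its duration.
; Sphere overlap launches the player up and along X, based on hit normal and facing direction.
; Unless IsHurt is set, it reduces health through MyGameMode and sets that flag briefly as a damage cooldown.
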(event OnComponentBeginOverlap(Sphere)
  (params (OverlappedComponent :type Primitive%20Component%20Object%20Reference) (OtherActor :type Actor%20Object%20Reference) (OtherComp :type Primitive%20Component%20Object%20Reference) (OtherBodyIndex :type Integer) (bFromSweep :type Boolean) (SweepResult :type Hit%20Result%20Structure%20%28by%20ref%29))
  (bind _x (Math|Vector|BreakVector (.normal SweepResult)))
  (bind _returnvalue (Game|Player|GetPlayerPawn 0))
  (bind _returnvalue_2 (* _x -4e+02))
  ;[1 1 1] Handle player hitting the object
  (if (== _returnvalue OtherActor)
    (bind _asplayer_bp (Utilities|Casting|CastToPlayerBP _returnvalue))
    ;;[1 1 1] Check Player direction to add force to that side, if still add to right
    (Math|Float|CompareFloat (.x (Math|Vector|GetForwardVector (Variables|/Script/Engine.Character|GetCapsuleComponent _asplayer_bp))) 0.0
      (:>
        (Character|LaunchCharacter _asplayer_bp (Math|Vector|MakeVector (+ _returnvalue_2 2e+02) 0.0 4e+02) true true :!label _label))
      (:==
        (goto _label))
      (:<
        (Character|LaunchCharacter _asplayer_bp (Math|Vector|MakeVector (- _returnvalue_2 2e+02) 0.0 4e+02) true true)))
    (if (not (Variables|/Game/Blueprints/PlayerBP.PlayerBP_C|GetisHurt _asplayer_bp))
      (bind _asmy_game_mode (Utilities|Casting|CastToMyGameMode (Game|GetGameMode)))
      (Default|ReduceHealth _asmy_game_mode)
      (Variables|/Game/Blueprints/PlayerBP.PlayerBP_C|SetisHurt _asplayer_bp true)
      (Utilities|FlowControl|Delay 0.5)
      (Variables|/Game/Blueprints/PlayerBP.PlayerBP_C|SetisHurt _asplayer_bp false))))

(fn ConstructionScript
  (bind _interptomovement (Variables|Default|GetInterpToMovement))
  (Variables|/Script/Engine.InterpToMovementComponent|SetDuration _interptomovement (Variables|Default|GetSpeed))
  (Variables|/Script/Engine.InterpToMovementComponent|SetControlPoints _interptomovement (Utilities|Array|MakeArray (Utilities|Struct|MakeInterpControlPoint (Variables|Default|GetPoint%20A) true) (Utilities|Struct|MakeInterpControlPoint (Variables|Default|GetPoint%20B) true))))