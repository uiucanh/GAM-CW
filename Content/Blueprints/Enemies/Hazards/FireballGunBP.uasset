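; FireballGunBP is a hazard that repeatedly fires FireBallBP projectiles.
; Tick feeds a Delay node, so the Delay variable sets the interval between shots.
; The Arrow's forward X, compared exactly to 1, decides whether the spawn point is offset toward positive or negative X.
; Each fireball takes the gun's rotation and receives SpeedOfFireball as its speed.
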(event Collision|EventActorBeginOverlap
  (params (OtherActor :type Actor%20Object%20Reference)))

(event EventTick
  (params (DeltaSeconds :type Float%20%28single-precision%29))
  (bind _returnvalue (Transformation|GetActorLocation))
  (bind _returnvalue_2 (Transformation|GetActorLocation))
  (bind _speedoffireball (Variables|Default|GetSpeedOfFireball))
  (Utilities|FlowControl|Delay (Variables|Default|GetDelay))
  (if (== (.x (Math|Vector|GetForwardVector (Variables|Default|GetArrow))) 1.0)
    (Game|SpawnActorfromClass "/Game/Blueprints/Enemies/Hazards/FireBallBP.FireBallBP_C" (Math|Transform|MakeTransform (Math|Vector|MakeVector (+ (.x _returnvalue_2) 5e+01) (.y _returnvalue_2) (.z _returnvalue_2)) (Transformation|GetActorRotation)) "Undefined" 0 _speedoffireball 0)
    (else
      (Game|SpawnActorfromClass "/Game/Blueprints/Enemies/Hazards/FireBallBP.FireBallBP_C" (Math|Transform|MakeTransform (Math|Vector|MakeVector (+ (.x _returnvalue) -5e+01) (.y _returnvalue) (.z _returnvalue)) (Transformation|GetActorRotation)) "Undefined" 0 _speedoffireball 0))))

(fn ConstructionScript)