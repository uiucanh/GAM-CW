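; FireBallBP is a projectile hazard that knocks back and damages the player on overlap, and is destroyed by overlapping anything else.
; The construction script copies a Speed variable into the ProjectileMovement speed limits.
; On player overlap it launches the character along the fireball's facing and hit normal, then, unless already hurt, reduces health through MyGameMode.
; It then hides itself and holds the player's IsHurt flag briefly before destroying itself.
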(event OnComponentBeginOverlap(RenderComponent)
  (params (OverlappedComponent :type Primitive%20Component%20Object%20Reference) (OtherActor :type Actor%20Object%20Reference) (OtherComp :type Primitive%20Component%20Object%20Reference) (OtherBodyIndex :type Integer) (bFromSweep :type Boolean) (SweepResult :type Hit%20Result%20Structure%20%28by%20ref%29))
  (bind _returnvalue (Game|Player|GetPlayerPawn 0))
  (bind _x (Math|Vector|BreakVector (.normal SweepResult)))
  (bind _returnvalue_2 (* _x -4e+02))
  ;[1 1 1] Handle collision with player, same mechanism as when hit by enemy, fireball is destroyed on contact
  (if (== OtherActor _returnvalue)
    (bind _asplayer_bp (Utilities|Casting|CastToPlayerBP _returnvalue))
    (if (> (.x (Math|Vector|GetForwardVector (Variables|Default|GetRenderComponent))) 0.0)
      (Character|LaunchCharacter _asplayer_bp (Math|Vector|MakeVector (+ _returnvalue_2 2e+02) 0.0 4e+02) true true)
      (else
        (Character|LaunchCharacter _asplayer_bp (Math|Vector|MakeVector (- _returnvalue_2 2e+02) 0.0 4e+02) true true)))
    (if (not (Variables|/Game/Blueprints/PlayerBP.PlayerBP_C|GetisHurt _asplayer_bp))
      (bind _asmy_game_mode (Utilities|Casting|CastToMyGameMode (Game|GetGameMode)))
      (Default|ReduceHealth _asmy_game_mode)
      (Variables|/Game/Blueprints/PlayerBP.PlayerBP_C|SetisHurt _asplayer_bp true)
      (Rendering|SetActorHiddenInGame true)
      (Collision|SetCollisionEnabled (Variables|Default|GetRenderComponent) "NoCollision")
      (Utilities|FlowControl|Delay 0.5)
      (Variables|/Game/Blueprints/PlayerBP.PlayerBP_C|SetisHurt _asplayer_bp false)
      (Actor|DestroyActor))
    (else
      (Actor|DestroyActor))))

(fn ConstructionScript
  (bind _speed (Variables|Default|GetSpeed))
  (bind _projectilemovement (Variables|Default|GetProjectileMovement))
  (Variables|/Script/Engine.ProjectileMovementComponent|SetInitialSpeed _projectilemovement _speed)
  (Variables|/Script/Engine.ProjectileMovementComponent|SetMaxSpeed _projectilemovement _speed))