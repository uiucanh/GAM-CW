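; 2D platformer enemy that patrols between two points through InterpToMovement, set up from PointA, PointB and Speed in the construction script.
; A hit on Top kills it: collision and movement stop, the death flipbook plays, the player is launched off it, then the actor is destroyed.
; Body overlap knocks the player back and reduces health via MyGameMode, throttled by a brief IsHurt window.
; Tick rotates the flipbook by X velocity.
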(event OnComponentBeginOverlap(Body)
  (params (OverlappedComponent :type Primitive%20Component%20Object%20Reference) (OtherActor :type Actor%20Object%20Reference) (OtherComp :type Primitive%20Component%20Object%20Reference) (OtherBodyIndex :type Integer) (bFromSweep :type Boolean) (SweepResult :type Hit%20Result%20Structure%20%28by%20ref%29))
  (bind _returnvalue (Game|Player|GetPlayerPawn 0))
  ;[1 1 1] When Player hit an enemy, reduce their health and knock them back
  (if (not (Variables|Default|GetisDead))
    (if (== _returnvalue OtherActor)
      (bind _asplayer_bp (Utilities|Casting|CastToPlayerBP _returnvalue))
      (Character|LaunchCharacter _asplayer_bp (Math|Vector|MakeVector (* (.X (Math|Vector|BreakVector (.normal SweepResult))) -4e+02) 0.0 4e+02) true true)
      ;[1 1 1] Deal damage to player health
      (if (not (Variables|/Game/Blueprints/PlayerBP.PlayerBP_C|GetisHurt _asplayer_bp))
        (bind _asmy_game_mode (Utilities|Casting|CastToMyGameMode (Game|GetGameMode)))
        (Default|ReduceHealth _asmy_game_mode)
        (Variables|/Game/Blueprints/PlayerBP.PlayerBP_C|SetisHurt _asplayer_bp true)
        (Utilities|FlowControl|Delay 0.5)
        (Variables|/Game/Blueprints/PlayerBP.PlayerBP_C|SetisHurt _asplayer_bp false)))))

(event OnComponentHit(Top)
  (params (HitComponent :type Primitive%20Component%20Object%20Reference) (OtherActor :type Actor%20Object%20Reference) (OtherComp :type Primitive%20Component%20Object%20Reference) (NormalImpulse :type Vector :default "0, 0, 0") (Hit :type Hit%20Result%20Structure%20%28by%20ref%29))
  (bind _returnvalue (* (.normal Hit) -3e+02))
  (bind (_x _y _z) (Math|Vector|BreakVector _returnvalue))
  ;[1 1 1] When player jumping on enemy, play death animation, destroy the mob and boost the player jump
  (Audio|PlaySound2D "/Game/Sound/EnemyHit.EnemyHit")
  (Variables|Default|SetisDead true)
  (Collision|SetCollisionEnabled (Variables|Default|GetTop) "NoCollision")
  (Components|Movement|StopMovementImmediately (Variables|Default|GetInterpToMovement))
  (Sprite|SetFlipbook (Variables|Default|GetPaperFlipbook) (Variables|Default|GetDeathFlipbook))
  (bind _asplayer_bp (Utilities|Casting|CastToPlayerBP (Game|Player|GetPlayerPawn 0)))
  (Character|LaunchCharacter _asplayer_bp (Math|Vector|MakeVector _x _y (+ _z 1e+02)) false false)
  (Utilities|FlowControl|Delay (Class|PaperFlipbookComponent|GetFlipbookLength (Variables|Default|GetPaperFlipbook)))
  (Actor|DestroyActor))

(event EventTick
  (params (DeltaSeconds :type Float%20%28single-precision%29))
  (bind _paperflipbook (Variables|Default|GetPaperFlipbook))
  ;[1 1 1] Change sprite direction
  (if (> (.x (Transformation|GetVelocity)) 0.0)
    (Transformation|SetWorldRotation _paperflipbook "0,180.000000, 0" false false)
    (else
      (Transformation|SetWorldRotation _paperflipbook "0, 0, 0" false false))))

(fn ConstructionScript
  (bind _interptomovement (Variables|Default|GetInterpToMovement))
  (Variables|/Script/Engine.InterpToMovementComponent|SetDuration _interptomovement (Variables|Default|GetSpeed))
  (Variables|/Script/Engine.InterpToMovementComponent|SetControlPoints _interptomovement (Utilities|Array|MakeArray (Utilities|Struct|MakeInterpControlPoint (Variables|Default|GetPoint%20A) true) (Utilities|Struct|MakeInterpControlPoint (Variables|Default|GetPoint%20B) true))))