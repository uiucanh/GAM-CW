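; BatBP is a bat enemy Blueprint that moves along a path through an InterpToMovement component.
; The construction script runs the parent's script, then appends PointC and PointD as relative control points and finalises the path.
; The event graph holds no active logic, so the Blueprint's own contribution is this path setup.
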(event EventBeginPlay)

(event Collision|EventActorBeginOverlap
  (params (OtherActor :type Actor%20Object%20Reference)))

(event EventTick
  (params (DeltaSeconds :type Float%20%28single-precision%29))
  (|CallParentFunction DeltaSeconds) ; This node is disabled and will not be called.\nDrag off pins to build functionality.
)

(fn ConstructionScript
  (bind _interptomovement (Variables|Default|GetInterpToMovement))
  (|CallParentFunction)
  (Utilities|Array|AppendArray (Variables|/Script/Engine.InterpToMovementComponent|GetControlPoints _interptomovement) (Utilities|Array|MakeArray (Utilities|Struct|MakeInterpControlPoint (Variables|Default|GetPoint%20C) true) (Utilities|Struct|MakeInterpControlPoint (Variables|Default|GetPoint%20D) true)))
  (Class|InterptoMovementComponent|FinaliseControlPoints _interptomovement))