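; Player character Blueprint for a 2D side-scrolling Paper2D platformer, handling input for lateral movement, jumping, crouching, climbing and interaction.
; Each tick, state checks pick the flipbook, prioritizing climb, duck and hurt over jump, walk and idle.
; Climbing switches to Flying movement and blocks lateral input until climb input ends, while control yaw flips to face movement.
; BeginPlay creates the health HUD, and landing re-arms the jump sound.
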(event Custom|UpdateAnimation
  (bind _returnvalue (Transformation|GetVelocity))
  (bind _sprite (Variables|Default|GetSprite))
  (bind _sprite_2 (Variables|Default|GetSprite))
  ;[1 1 1] Handle switching flipbook animations
  ;;[1 1 1] Check if player is jumping
  (if (Variables|Default|GetisClimbing)
    (Sprite|SetFlipbook (Variables|Default|GetSprite) "/Game/Sprites/Player/Flipbooks/Player_Climb_FB.Player_Climb_FB")
    (else
      ;;[1 1 1] Check if player is crouching
      (if (AI|Components|NavMovement|IsCrouching (Variables|Character|GetCharacterMovement))
        (Sprite|SetFlipbook _sprite_2 "/Game/Sprites/Player/Flipbooks/Player_Duck_FB.Player_Duck_FB")
        (elif (Variables|Default|GetisHurt)
          (Sprite|SetFlipbook _sprite_2 "/Game/Sprites/Player/Flipbooks/Player_Hurt_FB.Player_Hurt_FB")
          (elif (== (.Z (Math|Vector|BreakVector _returnvalue)) 0.0)
            (if (Variables|Default|GetisJumping)
              (Sprite|SetFlipbook _sprite "/Game/Sprites/Player/Flipbooks/Player_Jump_FB.Player_Jump_FB" :!label _label)
              (else
                (Sprite|SetFlipbook _sprite (select (> (Math|Vector|VectorLength _returnvalue) 0.0) "/Game/Sprites/Player/Flipbooks/Player_Walk_FB.Player_Walk_FB" "/Game/Sprites/Player/Flipbooks/Player_Idle_FB.Player_Idle_FB"))))
            (else
              (goto _label))))))))

(event Custom|EndClimbing
  ;[1 1 1] Handle ending climbing
  (if (Variables|Default|GetisClimbing)
    (Pawn|Components|CharacterMovement|SetMovementMode (Variables|Character|GetCharacterMovement) "MOVE_Walking" 0)
    (Variables|Default|SetisClimbing false)
    (Variables|Default|SetcanMoveRight true)))

(event EventTick
  (params (DeltaSeconds :type Float%20%28single-precision%29))
  ;[1 1 1] Handle switching flipbook animations
  (CallFunction|UpdateAnimation))

(event EventBeginPlay
  ;[1 1 1] Create the HUD widget
  (bind _returnvalue (UserInterface|CreateWidget "/Game/Blueprints/HUDs/MainWidget.MainWidget_C"))
  (bind _output_get (Variables|Default|SetHealthHUD _returnvalue))
  (UserInterface|Viewport|AddtoViewport _output_get 0))

(event EventOnLanded
  (params (Hit :type Hit%20Result%20Structure%20%28by%20ref%29))
  ;[1 1 1] Jump movement
  (Variables|Default|SetcanPlayJumpSound true))

(event Input|ActionEvents|InputActionJump
  (params (Key :type Key%20Structure))
  ;[1 1 1] Jump movement
  (:Pressed
    (Character|Jump)
    (Variables|Default|SetisJumping true)
    (if (Variables|Default|GetcanPlayJumpSound)
      (Audio|PlaySound2D "/Game/Sound/Jump_Cue.Jump_Cue")
      (Variables|Default|SetcanPlayJumpSound false)))
  (:Released
    (Character|StopJumping)
    (Variables|Default|SetisJumping false)))

(event Input|ActionEvents|InputActionInteract
  (params (Key :type Key%20Structure))
  ;[1 1 1] Interact with objects
  (:Pressed
    (Default|CallInteract)))

(event Input|ActionEvents|InputActionCrouch
  (params (Key :type Key%20Structure))
  (bind _canclimb (Variables|Default|GetcanClimb))
  ;[1 1 1] Crouch movement
  (:Pressed
    (if (not _canclimb)
      (Character|Crouch)
      (Components|Capsule|SetCapsuleHalfHeight (Variables|Collision|GetCapsuleComponent) 0.0 true)))
  (:Released
    (if (not _canclimb)
      (Character|UnCrouch))))

(event Input|AxisEvents|InputAxisClimbUp
  (params (AxisValue :type Float%20%28single-precision%29))
  (bind _charactermovement (Variables|Character|GetCharacterMovement))
  ;[1 1 1] Handle climbing movement
  ;;[1 1 1] Check for input
  (if (or (== AxisValue 1.0) (== AxisValue -1.0))
    (if (Variables|Default|GetcanClimb)
      ;;[1 1 1] Stop moving velocity
      (Variables|/Script/Engine.MovementComponent|SetVelocity _charactermovement (Math|Vector|MakeVector 0.0 (.y (Variables|/Script/Engine.MovementComponent|GetVelocity _charactermovement)) (.z (Variables|/Script/Engine.MovementComponent|GetVelocity _charactermovement))))
      (Variables|Default|SetisClimbing true)
      (Variables|Default|SetcanMoveRight false)
      (Pawn|Components|CharacterMovement|SetMovementMode _charactermovement "MOVE_Flying" 0)
      (Pawn|Input|AddMovementInput "0, 0,1.000000" AxisValue false))
    (else
      (CallFunction|EndClimbing))))

(event Input|AxisEvents|InputAxisLateralMovement
  (params (AxisValue :type Float%20%28single-precision%29))
  (bind _returnvalue (Pawn|GetController))
  ;[1 1 1] Lateral Movement
  (if (Variables|Default|GetcanMoveRight)
    (Pawn|Input|AddMovementInput "1.000000, 0, 0" AxisValue false)
    (Math|Float|CompareFloat AxisValue 0.0
      (:>
        (Pawn|SetControlRotation _returnvalue (Math|Rotator|MakeRotator 0.0 0.0 0.0)))
      (:<
        (Pawn|SetControlRotation _returnvalue (Math|Rotator|MakeRotator 0.0 0.0 1.8e+02))))))

(fn ConstructionScript)