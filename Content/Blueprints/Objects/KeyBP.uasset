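; KeyBP is a collectible key pickup that records which colored key has been obtained.
; When its PickUp component fires DeactivateDispatch, it plays a 2D pickup sound and sets the matching gold, red or blue flag on MyGameMode.
; The render component's sprite doubles as the key type: yellow means gold, red means red, and any other sprite counts as blue.
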(event DeactivateDispatch(PickUp)
  (bind _rendercomponent (Variables|Default|GetRenderComponent))
  (bind _returnvalue (Sprite|GetSprite _rendercomponent))
  (Audio|PlaySound2D "/Game/Sound/item_pickup.item_pickup")
  (bind _asmy_game_mode (Utilities|Casting|CastToMyGameMode (Game|GetGameMode)))
  (if (== _returnvalue "/Game/Sprites/Props/keyYellow_png.keyYellow_png")
    (Variables|/Game/Blueprints/MyGameMode.MyGameMode_C|SetGoldKeyObtained _asmy_game_mode true)
    (elif (== _returnvalue "/Game/Sprites/Props/keyRed_png.keyRed_png")
      (Variables|/Game/Blueprints/MyGameMode.MyGameMode_C|SetRedKeyObtained _asmy_game_mode true)
      (else
        (Variables|/Game/Blueprints/MyGameMode.MyGameMode_C|SetBlueKeyObtained _asmy_game_mode true)))))

(event EventBeginPlay
  (|CallParentFunction) ; This node is disabled and will not be called.\nDrag off pins to build functionality.
)

(event Collision|EventActorBeginOverlap
  (params (OtherActor :type Actor%20Object%20Reference)))

(event EventTick
  (params (DeltaSeconds :type Float%20%28single-precision%29)))

(fn ConstructionScript
  (|CallParentFunction))